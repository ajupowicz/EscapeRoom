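; Four-shelf safe riddle where opening shelves in the right order spawns a BP_Note, and a wrong one resets the shelves.
; InteractShelf slides a shelf out via timeline and records its index in UsersChoise, which Compare checks against RightOrder.
; A mismatch clears the choices and plays closing timelines.
; The completion count is unwired, so any matching prefix counts as success, and checks and spawning run on every timeline update.
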(event `/Game/Blueprints/BPI_Interaction.InteractShelf`
  (params (Shelf :type Integer))
  (switch `int` Shelf
    (:`0`
      (if (not (`self.bOpenedShelf`))
        (bind (_direction _open) (`Timeline|OpenShelf` :!via `PlayFromStart`)
          (:`Update`
            (`self.OpenShelfAnim` _open (`self.ShelfQuest`))
            (set `self.bOpenedShelf` true)
            (`KismetArrayLibrary.Array_AddUnique` (`self.UsersChoise`))
            (for (_array_element _array_index) (`self.UsersChoise`) :!label _label
              (`self.compare` _array_element _array_index
                (:`OutputPin`
                  (break))))
            (switch `int` (`self.bSameOrder`)
              (:`1`
                (bind _returnvalue (`|SpawnActorFromClass` "/Game/Blueprints/Items/BP_Note.BP_Note_C" (`self.Spawn Transform`) "Undefined" "MultiplyWithRoot" null null))
                (set `/Game/Blueprints/Items/BP_Note.ID` 1 _returnvalue))
              (:`2`
                ; wrong order shelf opened
                (`KismetArrayLibrary.Array_Clear` (`self.UsersChoise`))
                (for _index (range 4)
                  (switch `int` _index
                    (:`0`
                      (if (`self.bOpenedShelf`)
                        (bind (_direction_2 _open_2) (`Timeline|Timeline_2` :!via `PlayFromStart`)
                          (:`Update`
                            (`self.CloseShelfAnim` _open_2 (`self.ShelfQuest`))
                            (set `self.bOpenedShelf` false)))))
                    (:`1`
                      (if (`self.bOpenedShelf1`)
                        (bind (_direction_3 _open_3) (`Timeline|Timeline_3` :!via `PlayFromStart`)
                          (:`Update`
                            (`self.CloseShelfAnim` _open_3 (`self.Shelf1Quest`))
                            (set `self.bOpenedShelf1` false)))))
                    (:`2`
                      (if (`self.bOpenedShelf2`)
                        (bind (_direction_4 _open_4) (`Timeline|Timeline_4` :!via `PlayFromStart`)
                          (:`Update`
                            (`self.CloseShelfAnim` _open_4 (`self.Shelf2Quest`))
                            (set `self.bOpenedShelf2` false)))))
                    (:`3`
                      (if (`self.bOpenedShelf3`)
                        (bind (_direction_5 _open_5) (`Timeline|Timeline_5` :!via `PlayFromStart`)
                          (:`Update`
                            (`self.CloseShelfAnim` _open_5 (`self.Shelf3Quest`))
                            (set `self.bOpenedShelf3` false)))))))))))))
    (:`1`
      (if (not (`self.bOpenedShelf1`))
        (bind (_direction_6 _open_6) (`Timeline|Timeline` :!via `PlayFromStart`)
          (:`Update`
            (`self.OpenShelfAnim` _open_6 (`self.Shelf1Quest`))
            (set `self.bOpenedShelf1` true)
            (`KismetArrayLibrary.Array_AddUnique` (`self.UsersChoise`) 1)
            (goto _label)))))
    (:`2`
      (if (not (`self.bOpenedShelf2`))
        (bind (_direction_7 _open_7) (`Timeline|Timeline_0` :!via `PlayFromStart`)
          (:`Update`
            (`self.OpenShelfAnim` _open_7 (`self.Shelf2Quest`))
            (set `self.bOpenedShelf2` true)
            (`KismetArrayLibrary.Array_AddUnique` (`self.UsersChoise`) 2)
            (goto _label)))))
    (:`3`
      (if (not (`self.bOpenedShelf3`))
        (bind (_direction_8 _open_8) (`Timeline|Timeline_1` :!via `PlayFromStart`)
          (:`Update`
            (`self.OpenShelfAnim` _open_8 (`self.Shelf3Quest`))
            (set `self.bOpenedShelf3` true)
            (`KismetArrayLibrary.Array_AddUnique` (`self.UsersChoise`) 3)
            (goto _label)))))))

(fn `CloseShelfAnim`
  (params (Alpha :type "Float (double-precision)") (Shelf :type "SceneComponent Object Reference"))
  (bind (_relativelocation_x _relativelocation_y _relativelocation_z) (`KismetMathLibrary.BreakVector` (`SceneComponent.RelativeLocation` Shelf)))
  (`SceneComponent.K2_SetRelativeLocation` Shelf (`KismetMathLibrary.MakeVector` _relativelocation_x (`KismetMathLibrary.Lerp` 20.0 5.0 Alpha) _relativelocation_z) false false))

(fn `OpenShelfAnim`
  (params (Alpha :type "Float (double-precision)") (Shelf :type "SceneComponent Object Reference"))
  (bind (_relativelocation_x _relativelocation_y _relativelocation_z) (`KismetMathLibrary.BreakVector` (`SceneComponent.RelativeLocation` Shelf)))
  (`SceneComponent.K2_SetRelativeLocation` Shelf (`KismetMathLibrary.MakeVector` _relativelocation_x (`KismetMathLibrary.Lerp` 0.0 20.0 Alpha) _relativelocation_z) false false))

(fn `UserConstructionScript`)
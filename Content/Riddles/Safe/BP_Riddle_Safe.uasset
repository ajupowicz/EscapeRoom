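; Safe riddle actor that, on Interact, plays a lamp-triggered mechanism that shifts a painting out of the way.
; Three chained timelines run in sequence, each starting when the previous one finishes.
; The lamp mesh pitches down to -90 degrees, then the painting slides along local Y and rises along local Z.
; Each step lerps a single relative axis from its timeline track while preserving the other two.
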(event `/Game/Blueprints/BPI_Interaction.Interact`
  (params (`Player Character` :type "/Game/FirstPerson/Blueprints/BP_FirstPersonCharacter Object Reference"))
  (bind _lampmesh (`self.LampMesh`))
  (bind _painting (`self.Painting`))
  (bind _painting_2 (`self.Painting`))
  (bind (_relativelocation_x _relativelocation_y _relativelocation_z) (`KismetMathLibrary.BreakVector` (`SceneComponent.RelativeLocation` _painting_2)))
  (bind (_relativerotation_roll _relativerotation_pitch _relativerotation_yaw) (`KismetMathLibrary.BreakRotator` (`SceneComponent.RelativeRotation` _lampmesh)))
  (bind (_relativelocation_x_2 _relativelocation_y_2) (`KismetMathLibrary.BreakVector` (`SceneComponent.RelativeLocation` _painting)))
  ; Lamp rotate
  (bind (_direction _rotate) (`Timeline|Timeline`)
    (:`Update`
      (`SceneComponent.K2_SetRelativeRotation` _lampmesh (`KismetMathLibrary.MakeRotator` _relativerotation_roll (`KismetMathLibrary.Lerp` 0.0 -90.0 _rotate) _relativerotation_yaw) false false))
    (:`Finished`
      ; Painting Forward
      (bind (_direction_2 _basictrack) (`Timeline|Timeline_0`)
        (:`Update`
          (`SceneComponent.K2_SetRelativeLocation` _painting_2 (`KismetMathLibrary.MakeVector` _relativelocation_x (`KismetMathLibrary.Lerp` 0.0 5.0 _basictrack) _relativelocation_z) false false))
        (:`Finished`
          ; Painting Up
          (bind (_direction_3 _rotate_2) (`Timeline|Timeline_1`)
            (:`Update`
              (`SceneComponent.K2_SetRelativeLocation` _painting (`KismetMathLibrary.MakeVector` _relativelocation_x_2 _relativelocation_y_2 (`KismetMathLibrary.Lerp` 0.0 65.0 _rotate_2)) false false))))))))

(fn `UserConstructionScript`)
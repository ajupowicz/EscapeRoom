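; BP_Sanity is a zone actor that restores the player's sanity while they stand inside its sphere.
; On overlap, it starts a looping half-second timer that raises sanity and tells the player to pause its looped sanity drain.
; On exit, it unpauses the drain and pauses the timer.
; All changes reach player character 0 through message calls, so the player owns the sanity value.
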(event `self.Sphere.OnComponentBeginOverlap`
  (params (OverlappedComponent :type "PrimitiveComponent Object Reference") (OtherActor :type "Actor Object Reference") (OtherComp :type "PrimitiveComponent Object Reference") (OtherBodyIndex :type Integer) (bFromSweep :type Boolean) (SweepResult :type "HitResult Structure (by ref)"))
  (bind _returnvalue (`GameplayStatics.GetPlayerCharacter` 0))
  ; + Sanity
  (if (== OtherActor _returnvalue)
    (bind _returnvalue_2 (`KismetSystemLibrary.K2_SetTimerDelegate` (delegate `IncreaseSanity`) 0.5 true))
    (set `self.IncreaseSanityTimerHandle` _returnvalue_2)
    (message `/Game/Blueprints/BPI_Sanity.PauseReduceSanityLooped` _returnvalue)))

(event `IncreaseSanity`
  ; + Sanity
  (message `/Game/Blueprints/BPI_Sanity.IncreaseSanity` (`GameplayStatics.GetPlayerCharacter` 0) 1.0))

(event `self.Sphere.OnComponentEndOverlap`
  (params (OverlappedComponent :type "PrimitiveComponent Object Reference") (OtherActor :type "Actor Object Reference") (OtherComp :type "PrimitiveComponent Object Reference") (OtherBodyIndex :type Integer))
  (bind _returnvalue (`GameplayStatics.GetPlayerCharacter` 0))
  (bind _increasesanitytimerhandle (`self.IncreaseSanityTimerHandle`))
  ; - Sanity
  (if (== OtherActor _returnvalue)
    (message `/Game/Blueprints/BPI_Sanity.UnpauseReduceSanityLooped` _returnvalue)
    (if (`KismetSystemLibrary.K2_IsValidTimerHandle` _increasesanitytimerhandle)
      (`KismetSystemLibrary.K2_PauseTimerHandle` _increasesanitytimerhandle))))

(fn `UserConstructionScript`)
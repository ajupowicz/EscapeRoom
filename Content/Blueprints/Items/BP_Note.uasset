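; BP_Note is a note item actor that picks its static mesh when play begins.
; BeginPlay switches on ID and, for each of four values (0 to 3), looks up a row through a separate data table row handle.
; When the row is found, its Mesh is applied to NoteMesh; the construction script is empty.
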(event `self.ReceiveBeginPlay`
  (bind (_dtmeshes_2_datatable _dtmeshes_2_rowname) (break `DataTableRowHandle` (`self.DTMeshes_2`)))
  (bind (_dtmeshes_1_datatable _dtmeshes_1_rowname) (break `DataTableRowHandle` (`self.DTMeshes_1`)))
  (bind (_dtmeshes_datatable _dtmeshes_rowname) (break `DataTableRowHandle` (`self.DTMeshes`)))
  (bind (_dtmeshes_0_datatable _dtmeshes_0_rowname) (break `DataTableRowHandle` (`self.DTMeshes_0`)))
  (switch `int` (`self.ID`)
    (:`0`
      (bind _returnvalue (`|GetDataTableRow` _dtmeshes_datatable _dtmeshes_rowname)
        (:`then`
          (`StaticMeshComponent.SetStaticMesh` (`self.NoteMesh`) (`.Mesh_10_654CDA484BEE1F9105D85B9FD75CB48D` (break `/Game/DataTable/Struct_Notes` _returnvalue))))))
    (:`1`
      (bind _returnvalue_2 (`|GetDataTableRow` _dtmeshes_0_datatable _dtmeshes_0_rowname)
        (:`then`
          (`StaticMeshComponent.SetStaticMesh` (`self.NoteMesh`) (`.Mesh_10_654CDA484BEE1F9105D85B9FD75CB48D` (break `/Game/DataTable/Struct_Notes` _returnvalue_2))))))
    (:`2`
      (bind _returnvalue_3 (`|GetDataTableRow` _dtmeshes_1_datatable _dtmeshes_1_rowname)
        (:`then`
          (`StaticMeshComponent.SetStaticMesh` (`self.NoteMesh`) (`.Mesh_10_654CDA484BEE1F9105D85B9FD75CB48D` (break `/Game/DataTable/Struct_Notes` _returnvalue_3))))))
    (:`3`
      (bind _returnvalue_4 (`|GetDataTableRow` _dtmeshes_2_datatable _dtmeshes_2_rowname)
        (:`then`
          (`StaticMeshComponent.SetStaticMesh` (`self.NoteMesh`) (`.Mesh_10_654CDA484BEE1F9105D85B9FD75CB48D` (break `/Game/DataTable/Struct_Notes` _returnvalue_4))))))))

(fn `UserConstructionScript`)
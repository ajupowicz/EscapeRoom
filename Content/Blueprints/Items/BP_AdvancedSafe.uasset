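; Two-stage interactive safe: a combination dial opens the large door, then a PIN keypad opens the small inner door.
; Interacting blends to the current door's camera and swaps input from character to safe.
; Held A/D loop timers turn the dial in timeline-smoothed steps, matching code numbers in alternating directions and resetting on wrong turns.
; Keypad widget events update the PIN display, while timelines swing the doors open.
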(event `self.ReceiveBeginPlay`
  ; BEGIN PLAY
  (`self.Reset Circle Code`)
  (`self.Keyboard Binds`))

(event `/Game/Blueprints/BPI_Interaction.Interact`
  (params (`Player Character` :type "/Game/FirstPerson/Blueprints/BP_FirstPersonCharacter Object Reference"))
  (bind _returnvalue (`GameplayStatics.GetPlayerController` 0))
  ; INTERACTION
  (if (not (`self.bDoorsOpening`))
    ; Show the cursor and switch to UI mode depending on the door
    (if (`self.bOpenedLargeDoor`)
      (set `PlayerController.bShowMouseCursor` true _returnvalue)
      (`WidgetBlueprintLibrary.SetInputMode_GameAndUIEx` _returnvalue null "DoNotLock" false))
    (`self.InteractDoor`)))

(event `InteractDoor`
  (bind _returnvalue (`GameplayStatics.GetPlayerController` 0))
  (bind _returnvalue_2 (`GameplayStatics.GetPlayerController` 0))
  ; INTERACTION DOOR
  (if (`self.bIsActive?`) :!label _label
    ; Hide/Show the character during transitions
    (bind _asbp_first_person_character (cast `/Game/FirstPerson/Blueprints/BP_FirstPersonCharacter` (`GameplayStatics.GetPlayerCharacter` 0)))
    (`SceneComponent.SetVisibility` (`/Game/FirstPerson/Blueprints/BP_FirstPersonCharacter.FirstPersonMesh` _asbp_first_person_character) true false)
    ; Move the camera back to the character
    (`PlayerController.SetViewTargetWithBlend` (`GameplayStatics.GetPlayerController` 0) (`GameplayStatics.GetPlayerCharacter` 0) (`self.End Blend Time`) "VTBlend_Cubic" 1.0 false)
    ; Wait for the camera transition animation to finish before restoring player control
    (`KismetSystemLibrary.Delay` (`self.End Blend Time`))
    ; Restore control back to the player
    (`self.EnableInput` (`GameplayStatics.GetPlayerCharacter` 0) _returnvalue_2)
    (`self.DisableInput` _returnvalue_2)
    (set `self.bIsActive?` false)
    (bind _asbp_first_person_character_2 (cast `/Game/FirstPerson/Blueprints/BP_FirstPersonCharacter` (`GameplayStatics.GetPlayerCharacter` 0)))
    (`/Game/FirstPerson/Blueprints/BP_FirstPersonCharacter.ShowInventory` _asbp_first_person_character_2)
    (else
      (bind _asbp_first_person_character_3 (cast `/Game/FirstPerson/Blueprints/BP_FirstPersonCharacter` (`GameplayStatics.GetPlayerCharacter` 0)))
      (`SceneComponent.SetVisibility` (`/Game/FirstPerson/Blueprints/BP_FirstPersonCharacter.FirstPersonMesh` _asbp_first_person_character_3) false false)
      ; Move the character's camera to the safe's camera
      (`PlayerController.SetViewTargetWithBlend` (`GameplayStatics.GetPlayerController` 0) (select `bool` (`self.bOpenedLargeDoor`) :`false` (`self.Camera_LargeDoor`) :`true` (`self.Camera_SmallDoor`) :!type "Actor Object Reference") (`self.Start Blend Time`) "VTBlend_Cubic" 1.0 false)
      (bind _asbp_first_person_character_4 (cast `/Game/FirstPerson/Blueprints/BP_FirstPersonCharacter` (`GameplayStatics.GetPlayerCharacter` 0)))
      (`/Game/FirstPerson/Blueprints/BP_FirstPersonCharacter.HideInventory` _asbp_first_person_character_4)
      ; Disable player input immediately to prevent character movement after interacting
      (`self.DisableInput` (`GameplayStatics.GetPlayerCharacter` 0) _returnvalue)
      ; Add a delay to prevent the player from spamming the interaction button
      (`KismetSystemLibrary.Delay` (`self.Start Blend Time`))
      ; Enable input for the safe actor to allow the player to exit interaction mode
      (`self.EnableInput` _returnvalue)
      (set `self.bIsActive?` true)))
  (`SceneComponent.SetVisibility` (`self.PINCodeKeyboard`) (`self.bOpenedLargeDoor`) false))

(event `EnhancedInput|/Game/Input/Actions/IA_Interaction`
  (params (ActionValue :type Boolean) (ElapsedSeconds :type "Float (double-precision)") (TriggeredSeconds :type "Float (double-precision)") (InputAction :type "InputAction Object Reference" :default "/Game/Input/Actions/IA_Interaction.IA_Interaction"))
  ; Exit the interaction mode with the safe
  (:`Triggered`
    (goto _label)))

(event `Open Small Door`
  (bind _returnvalue (`GameplayStatics.GetPlayerController` 0))
  ; Open Small Door
  (`self.InteractDoor`)
  (set `self.bDoorsOpening` true)
  (set `PlayerController.bShowMouseCursor` false _returnvalue)
  (`WidgetBlueprintLibrary.SetInputMode_GameOnly` _returnvalue)
  (`KismetSystemLibrary.Delay` (`self.End Blend Time`))
  (bind (_direction _alpha) (`Timeline|TL_OpenSmallDoor` :!via `PlayFromStart`)
    (:`Update`
      (`SceneComponent.K2_SetRelativeRotation` (`self.SM_Safe_CodeDoor`) (`KismetMathLibrary.MakeRotator` 0.0 0.0 (`KismetMathLibrary.Lerp` 0.0 -125.0 _alpha)) false false))))

(event `Circle Rotation Left`
  (bind _angle (`self.Angle`))
  (bind _relativerotation_roll (`KismetMathLibrary.BreakRotator` (`SceneComponent.RelativeRotation` (`self.SM_Safe_Code`))))
  ; Safe Code Rotation
  (if (`self.bCanRotation`)
    (set `self.bCanRotation` false)
    (set `self.bRotationDirection` true)
    ; Rotation Speed
    (`TimelineComponent.SetPlayRate` (`self.TL_Rotation`) (`self.Safe Circle Rotation Speed`) :!label _label_2)
    ; Makes the rotation smooth using a timeline, rotating the static mesh from its current position by ±4.5 degrees
    (bind (_direction _alpha) (`Timeline|TL_Rotation` :!via `PlayFromStart`)
      (:`Update`
        (`SceneComponent.K2_SetRelativeRotation` (`self.SM_Safe_Code`) (`KismetMathLibrary.MakeRotator` (`KismetMathLibrary.Lerp` (`self.Angle`) (`KismetMathLibrary.SelectFloat` (- _angle 4.5) (+ _angle 4.5) (`self.bRotationDirection`)) _alpha) 0.0 90.0) false false))
      (:`Finished`
        ; Get the current rotation of the static mesh
        (bind _output_get (set `self.Angle` (`KismetMathLibrary.SelectFloat` _relativerotation_roll (+ _relativerotation_roll 360.0) (> _relativerotation_roll 0.0))))
        ; Get current code number
        (set `self.CurrentNum` (/ _output_get 4.5))
        (set `self.bCanRotation` true)
        ; Check if the rotation is in the correct direction
        (if (== (`self.bRotationDirection`) (`self.bCorrectDirection`))
          ; Check if the first digit of the code is entered correctly
          (if (== (`self.CurrentNum`) (`|GetArrayItem` (`self.Safe Circle Code`) (`self.CircleCodeIndex`)))
            ; Change the required rotation direction
            (set `self.bCorrectDirection` (not (`self.bCorrectDirection`)))
            ; Move to the next digit of the code
            (set `self.CircleCodeIndex` (+ (`self.CircleCodeIndex`) 1))
            ; Check if the entered number is the last one
            (if (== (`self.CircleCodeIndex`) (`KismetArrayLibrary.Array_Length` (`self.Safe Circle Code`)))
              (`self.Open Large Door`)))
          (else
            ; If the rotation direction is incorrect, the progress will be reset
            (`self.Reset Circle Code`)))))))

(event `Circle Rotation Right`
  ; Safe Code Rotation
  (if (`self.bCanRotation`)
    (set `self.bCanRotation` false)
    (set `self.bRotationDirection` false)
    (goto _label_2)))

(event `Check PIN Code`
  (params (Code :type String))
  ; Check PIN Code
  (if (`KismetStringLibrary.EqualEqual_StrStr` Code (`self.PIN Code`))
    (`self.Open Small Door`)
    (bind _asbp_first_person_character (cast `/Game/FirstPerson/Blueprints/BP_FirstPersonCharacter` (`GameplayStatics.GetPlayerCharacter` 0)))
    (`/Game/FirstPerson/Blueprints/BP_FirstPersonCharacter.ShowInventory` _asbp_first_person_character)
    (else
      ; Incorrect
      (bind _aswb_safe_pincode (cast `/Game/Blueprints/WB_SafePINCode` (`WidgetComponent.GetWidget` (`self.PINCode`))))
      (`TextBlock.SetText` (`/Game/Blueprints/WB_SafePINCode.T_PINCode` _aswb_safe_pincode) (`KismetTextLibrary.Conv_StringToText` ""))
      (set `/Game/Blueprints/WB_SafeKeyboard.Code` "" (cast `/Game/Blueprints/WB_SafeKeyboard` (`WidgetComponent.GetWidget` (`self.PINCodeKeyboard`)) :!pure true)))))

(event `Reset Circle Code`
  ; Set the direction in which the rotation should start
  (bind _output_get (set `self.bRotationDirection` (`self.bStartDirection`)))
  (set `self.bCorrectDirection` _output_get)
  (set `self.CircleCodeIndex` 0))

(event `Key|A`
  (params (Key :type "Key Structure"))
  (bind _bopenedlargedoor (`self.bOpenedLargeDoor`))
  ; SAFE CIRCLE CODE - Starts a timer to loop the rotation while the button is held
  (:`Pressed`
    (if (not _bopenedlargedoor)
      (bind _returnvalue (`KismetSystemLibrary.K2_SetTimer` null "Circle Rotation Left" 0.01 true))))
  (:`Released`
    (if (not _bopenedlargedoor)
      (`KismetSystemLibrary.K2_ClearAndInvalidateTimerHandle` _returnvalue))))

(event `Keyboard Binds`
  (bind _aswb_safe_keyboard (cast `/Game/Blueprints/WB_SafeKeyboard` (`WidgetComponent.GetWidget` (`self.PINCodeKeyboard`)) :!pure true))
  ; Keyboard Binds
  (add `/Game/Blueprints/WB_SafeKeyboard.ED_Update` _aswb_safe_keyboard (delegate `Update PINCode`))
  (set `/Game/Blueprints/WB_SafeKeyboard.PINCodeMaxNum` (`self.PINCodeMaxNum`) _aswb_safe_keyboard)
  (add `/Game/Blueprints/WB_SafeKeyboard.ED_Enter` _aswb_safe_keyboard (`|CreateDelegate` :!event `Check PIN Code`)))

(event `Open Large Door`
  ; Open Large Door
  (`self.InteractDoor`)
  (`KismetSystemLibrary.Delay` (`self.End Blend Time`))
  (set `self.bOpenedLargeDoor` true)
  (bind (_direction _alpha _handle) (`Timeline|TL_OpenDoor` :!via `PlayFromStart`)
    (:`Update`
      (`SceneComponent.K2_SetRelativeRotation` (`self.SM_Safe_Door`) (`KismetMathLibrary.MakeRotator` 0.0 0.0 (`KismetMathLibrary.Lerp` 0.0 -125.0 _alpha)) false false)
      (`SceneComponent.K2_SetRelativeRotation` (`self.SM_Safe_Handle`) (`KismetMathLibrary.MakeRotator` 0.0 (`KismetMathLibrary.Lerp` 0.0 -30.0 _handle)) false false))))

(event `Key|D`
  (params (Key :type "Key Structure"))
  (bind _bopenedlargedoor (`self.bOpenedLargeDoor`))
  ; SAFE CIRCLE CODE - Starts a timer to loop the rotation while the button is held
  (:`Pressed`
    (if (not _bopenedlargedoor)
      (bind _returnvalue (`KismetSystemLibrary.K2_SetTimer` null "Circle Rotation Right" 0.01 true))))
  (:`Released`
    (if (not _bopenedlargedoor)
      (`KismetSystemLibrary.K2_ClearAndInvalidateTimerHandle` _returnvalue))))

(event `Update PINCode`
  (params (Code :type String))
  ; Update PIN Code
  (bind _aswb_safe_pincode (cast `/Game/Blueprints/WB_SafePINCode` (`WidgetComponent.GetWidget` (`self.PINCode`))))
  (`TextBlock.SetText` (`/Game/Blueprints/WB_SafePINCode.T_PINCode` _aswb_safe_pincode) (`KismetTextLibrary.Conv_StringToText` Code)))

(fn `UserConstructionScript`)
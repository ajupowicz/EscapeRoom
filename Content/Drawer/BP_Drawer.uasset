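; BP_Drawer is an interactable puzzle drawer that reports its index to a puzzle controller when clicked.
; BeginPlay caches the mesh's closed position and derives an open position from a fixed Y offset.
; Interact sets a one-click guard, notifies the controller and plays a timeline that lerps the mesh between both positions.
; ResetDrawer waits briefly, clears the guard and snaps the mesh back to closed.
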(event `ResetDrawer`
  ; Reset sequence and animation
  (`KismetSystemLibrary.Delay` 0.5)
  (set `self.bWasClicked` false)
  (`SceneComponent.K2_SetRelativeLocation` (`self.StaticMesh`) (`self.ClosedLocation`) false false))

(event `self.ReceiveBeginPlay`
  ; Setting the laction of drawers
  (set `self.ClosedLocation` (`SceneComponent.RelativeLocation` (`self.StaticMesh`)))
  (set `self.OpenLocation` (+ (`self.ClosedLocation`) (0.0 23.0 0.0))))

(event `/Game/Blueprints/BPI_Interaction.Interact`
  (params (`Player Character` :type "/Game/FirstPerson/Blueprints/BP_FirstPersonCharacter Object Reference"))
  (if (not (`self.bWasClicked`))
    (set `self.bWasClicked` true)
    (`/Game/Drawer/BP_DrawerPuzzleController.OnDrawerClicked` (`self.PuzzleControllerRef `) (`self.DrawerIndex`))
    ; Animation
    (bind (_direction _newtrack_0) (`Timeline|Oś czasu` :!via `PlayFromStart`)
      (:`Update`
        (`SceneComponent.K2_SetRelativeLocation` (`self.StaticMesh`) (`KismetMathLibrary.VLerp` (`self.OpenLocation`) (`self.ClosedLocation`) _newtrack_0) false false)))))

(fn `UserConstructionScript`)
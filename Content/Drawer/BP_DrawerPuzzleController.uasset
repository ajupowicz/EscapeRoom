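; BP_DrawerPuzzleController runs a puzzle where three drawers must be clicked in a set order.
; On BeginPlay it gathers every BP_Drawer, then records each clicked index and, on the third click, compares the sequence against CorrectOrder.
; A match starts the action on RefDrawerWin; a mismatch adds an audio component and resets the click state and all drawers.
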(event `self.ReceiveBeginPlay`
  (bind _outactors (`GameplayStatics.GetAllActorsOfClass` "/Game/Drawer/BP_Drawer.BP_Drawer_C"))
  (set `self.Drawers` _outactors))

(event `OnDrawerClicked`
  (params (DrawerIndex :type Integer))
  (`KismetArrayLibrary.Array_Add` (`self.ClickedOrder`) DrawerIndex)
  (`KismetSystemLibrary.PrintString` (`KismetStringLibrary.Conv_IntToString` DrawerIndex))
  (set `self.ClickCount` (+ (`self.ClickCount`) 1))
  (if (== (`self.ClickCount`) 3)
    (set `self.IsSequenceCorrect` true)
    (for _index (range (`self.ClickCount`))
      (if (not (== (`|GetArrayItem` (`self.ClickedOrder`) _index) (`|GetArrayItem` (`self.CorrectOrder`) _index)))
        (set `self.IsSequenceCorrect` false)
        (break)))
    (if (`self.IsSequenceCorrect`)
      (`/Game/Drawer/BP_DrawerWin.StartAction` (`self.RefDrawerWin`))
      (else
        (`AddComponent|NODE_AddAudioComponent-0`)
        (`self.ResetPuzzle()`)))))

(fn `ResetPuzzle()`
  (`KismetArrayLibrary.Array_Clear` (`self.ClickedOrder`))
  (set `self.ClickCount` 0)
  (set `self.IsSequenceCorrect` false)
  (for _array_element (`self.Drawers`)
    (`/Game/Drawer/BP_Drawer.ResetDrawer` _array_element)))

(fn `UserConstructionScript`)
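; BP_DrawerWin is a drawer that slides open and holds a photo mesh that becomes a pickup.
; StartAction adds an audio component and plays a timeline that lerps the drawer mesh along local Y, flagging it open as it moves.
; Once that flag is set, Interact spawns the configured pickup class at the photo's transform, then hides the photo and disables its collision.
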(event `StartAction`
  (bind _staticmesh (`self.StaticMesh`))
  (bind (_relativelocation_x _relativelocation_y _relativelocation_z) (`KismetMathLibrary.BreakVector` (`SceneComponent.RelativeLocation` _staticmesh)))
  (`AddComponent|NODE_AddAudioComponent-0`)
  (bind (_direction _newtrack_0) (`Timeline|Oś czasu`)
    (:`Update`
      (`SceneComponent.K2_SetRelativeLocation` _staticmesh (`KismetMathLibrary.MakeVector` _relativelocation_x (`KismetMathLibrary.Lerp` 0.0 23.0 _newtrack_0) _relativelocation_z) false false)
      (set `self.Isopen` true))))

(event `/Game/Blueprints/BPI_Interaction.Interact`
  (params (`Player Character` :type "/Game/FirstPerson/Blueprints/BP_FirstPersonCharacter Object Reference"))
  (if (`self.Isopen`)
    (`|SpawnActorFromClass` (`self.PickupItemClass`) (`SceneComponent.K2_GetComponentToWorld` (`self.SM_Photo_M`)) "Undefined" "MultiplyWithRoot" null null)
    (`SceneComponent.SetHiddenInGame` (`self.SM_Photo_M`) true false)
    (`PrimitiveComponent.SetCollisionEnabled` (`self.SM_Photo_M`) "NoCollision")))

(fn `UserConstructionScript`)